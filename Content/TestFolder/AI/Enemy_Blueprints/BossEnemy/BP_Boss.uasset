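; BP_Boss is a boss enemy Blueprint in a test AI folder that stubs out the boss's attacks.
; Custom events for two fist shots, a laser and a primary melee attack only print debug strings, with no real attack logic yet.
; GetIdealRange returns fixed attack, defend and charge radii, with charge set farther out than the other two.
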(event `FireFist1`
  (`KismetSystemLibrary.PrintString` "Fist One Fired"))

(event `FireFist2`
  (`KismetSystemLibrary.PrintString` "Fist 2 Fired"))

(event `LaserAttack`
  (`KismetSystemLibrary.PrintString` "Lase Fired"))

(event `/Game/TestFolder/AI/Logic/BPI_EnemyInterface.PrimaryAttack`
  (`KismetSystemLibrary.PrintString` "Melee Attack"))

(fn `GetIdealRange`
  (returns (AttackRadius :type "Float (double-precision)") (DefendRadius :type "Float (double-precision)") (ChargeRadius :type "Float (double-precision)"))
  (return 200.0 200.0 700.0))

(fn `UserConstructionScript`
  (`parent.UserConstructionScript`))