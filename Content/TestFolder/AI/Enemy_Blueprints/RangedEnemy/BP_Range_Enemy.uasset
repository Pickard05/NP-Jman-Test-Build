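; Ranged enemy character that supplies its own attack, movement speeds and ideal combat ranges to the AI.
; PrimaryAttack plays a pistol aim montage and, on its notify, has the enemy attacks component fire from the Muzzle socket at the AI controller's attack target.
; Montage completion or interruption signals attack end.
; SetMovementSpeed maps movement types to walk speed, and GetIdealRange returns attack and defend radii, with zero charge radius.
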(event `/Game/TestFolder/AI/Logic/BPI_EnemyInterface.PrimaryAttack`
  (`KismetSystemLibrary.PrintString` "Attack Performed")
  (bind _notifyname (`|PlayMontage` (`self.Mesh`) "/Game/TestFolder/SimpleProjectile/PistolAim_UE_Montage.PistolAim_UE_Montage" 2.0)
    (:`OnCompleted`
      (`self.OnAttackEnd` :!label _label))
    (:`OnInterrupted`
      (goto _label))
    (:`OnNotifyBegin`
      (switch `name` _notifyname
        (:`Fire`
          (bind _asai_controller (cast `/Game/TestFolder/AI/Enemy_Blueprints/AI_Controller` (`AIBlueprintHelperLibrary.GetAIController` self)))
          (bind _attack_target (`/Game/TestFolder/AI/Enemy_Blueprints/AI_Controller.Attack Target` _asai_controller)
            (:`then`
              (`/Game/TestFolder/SimpleProjectile/BPC_EnemyAttacks.RangedEnemyAttack` (`self.BPC_EnemyAttacks`) (`SceneComponent.GetSocketTransform` (`self.Mesh`) "Muzzle" "RTS_World") _attack_target))
            (:`else`)))))))

(fn `GetIdealRange`
  (returns (AttackRadius :type "Float (double-precision)") (DefendRadius :type "Float (double-precision)") (ChargeRadius :type "Float (double-precision)"))
  (return 600.0 600.0 0.0))

(fn `SetMovementSpeed`
  (params (`Movement Type` :type "/Game/TestFolder/AI/Logic/Enumerations/E_EnemyMovementSpeed Enum" :default "NewEnumerator0"))
  (returns (`Movement Speed` :type "Float (double-precision)"))
  (bind _output_get (set `CharacterMovementComponent.MaxWalkSpeed` (select `/Game/TestFolder/AI/Logic/Enumerations/E_EnemyMovementSpeed` `Movement Type` :`NewEnumerator1` 200.0 :`NewEnumerator2` 300.0 :`NewEnumerator3` 500.0) (`self.CharacterMovement`)))
  (return _output_get))

(fn `UserConstructionScript`
  (`parent.UserConstructionScript`))