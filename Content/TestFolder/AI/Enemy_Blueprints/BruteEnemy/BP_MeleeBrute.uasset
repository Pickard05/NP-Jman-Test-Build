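; Melee brute enemy, a child Blueprint that supplies its own movement speeds, including a fast charge, and attack, defend and charge ranges.
; Primary attack is a placeholder that prints a message, signals completion, then delays AttackEnd to slow attack token distribution.
; Pushback box-traces ahead for pawns and, on any hit, launches the player cached at BeginPlay along the brute's forward vector with an explosion effect.
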(event `self.ReceiveBeginPlay`
  (`parent.ReceiveBeginPlay`)
  (bind _asplayer (cast `/Game/TestFolder/Player/Player` (`GameplayStatics.GetPlayerCharacter` 0)))
  (set `self.As Player` _asplayer))

(event `self.PrimaryAttack`
  (params (AttackTarget :type "Actor Object Reference"))
  (`parent.PrimaryAttack` AttackTarget)
  (`KismetSystemLibrary.PrintString` "Attack Performed")
  (`self.OnAttackEnd`)
  ;[1 1 1] Slow the token distrubution down while theres no attack in
  (`KismetSystemLibrary.Delay` 2.0)
  (`self.AttackEnd` AttackTarget))

(event `Pushback`
  (bind _returnvalue (`self.GetActorForwardVector`))
  (bind _returnvalue_2 (`self.GetActorForwardVector`))
  (bind _boxpushbackspawnpoint (`self.BoxPushbackSpawnPoint`))
  (bind _returnvalue_3 (`SceneComponent.K2_GetComponentLocation` _boxpushbackspawnpoint))
  (bind (_returnvalue_x _returnvalue_y) (`KismetMathLibrary.BreakVector` (* _returnvalue 1000.0)))
  (bind (_outhit _returnvalue_4) (`KismetSystemLibrary.BoxTraceSingleForObjects` (+ _returnvalue_3 (* _returnvalue_2 100.0)) (+ _returnvalue_3 (* _returnvalue_2 200.0)) (20.0 50.0 50.0) (`SceneComponent.K2_GetComponentRotation` _boxpushbackspawnpoint) (`|MakeArray` "ObjectTypeQuery3" :!type "EObjectTypeQuery Enum") false (`|MakeArray` self :!type "Actor Object Reference") "ForDuration"))
  (if _returnvalue_4
    (`self.LaunchCharacter` (`self.As Player`) (`KismetMathLibrary.MakeVector` _returnvalue_x _returnvalue_y 2.0) false true)
    (`GameplayStatics.SpawnEmitterAtLocation` "/Game/StarterContent/Particles/P_Explosion.P_Explosion" (+ (`self.K2_GetActorLocation`) (* _returnvalue 50.0)) (`self.K2_GetActorRotation`))))

(fn `GetIdealRange`
  (returns (AttackRadius :type "Float (double-precision)") (DefendRadius :type "Float (double-precision)") (ChargeRadius :type "Float (double-precision)"))
  (return 200.0 350.0 1000.0))

(fn `SetMovementSpeed`
  (params (`Movement Type` :type "/Game/TestFolder/AI/Logic/Enumerations/E_EnemyMovementSpeed Enum" :default "NewEnumerator0"))
  (returns (`Movement Speed` :type "Float (double-precision)"))
  (bind _output_get (set `CharacterMovementComponent.MaxWalkSpeed` (select `/Game/TestFolder/AI/Logic/Enumerations/E_EnemyMovementSpeed` `Movement Type` :`NewEnumerator1` 150.0 :`NewEnumerator2` 300.0 :`NewEnumerator3` 500.0 :`NewEnumerator4` 1500.0) (`self.CharacterMovement`)))
  (return _output_get))

(fn `UserConstructionScript`
  (`parent.UserConstructionScript`))