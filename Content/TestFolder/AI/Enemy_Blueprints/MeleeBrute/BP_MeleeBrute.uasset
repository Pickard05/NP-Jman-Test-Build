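; BP_MeleeBrute is a melee enemy character that supplies movement and range behavior, apparently for AI use.
; SetMovementSpeed maps a movement type to the CharacterMovement max walk speed, including a very fast Charge tier, and returns it.
; GetIdealRange returns fixed attack, defend and charge radii.
; PrimaryAttack is a placeholder that prints a debug string and jumps, while BeginPlay, overlap and Tick are disabled.
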(event `/Game/TestFolder/AI/Logic/BPI_EnemyInterface.PrimaryAttack`
  (`KismetSystemLibrary.PrintString` "Pow Pow")
  (`self.Jump`))

(fn `GetIdealRange`
  (returns (AttackRadius :type "Float (double-precision)") (DefendRadius :type "Float (double-precision)") (ChargeRadius :type "Float (double-precision)"))
  (return 250.0 300.0 1000.0))

(fn `SetMovementSpeed`
  (params (`Movement Type` :type "/Game/TestFolder/AI/Logic/Enumerations/E_EnemyMovementSpeed Enum" :default "NewEnumerator0"))
  (returns (`Movement Speed` :type "Float (double-precision)"))
  (bind _output_get (set `CharacterMovementComponent.MaxWalkSpeed` (select `/Game/TestFolder/AI/Logic/Enumerations/E_EnemyMovementSpeed` `Movement Type` :`NewEnumerator1` 150.0 :`NewEnumerator2` 300.0 :`NewEnumerator3` 500.0 :`NewEnumerator4` 2000.0) (`self.CharacterMovement`)))
  (return _output_get))

(fn `UserConstructionScript`
  (`parent.UserConstructionScript`))