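; Actor component that provides enemy attacks: a ranged projectile shot and a launched fist.
; Each attack event spawns its actor (BP_Tier1_Projectile or BP_Fist) at a given transform and target, owned by the component's owner, and binds to its impact dispatcher.
; On impact, either attack applies fixed damage to the hit actor, fires the OnAttackEnded dispatcher and prints the damage result.
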(event `RangedEnemyAttack`
  (params (SpawnTransform :type "Transform Structure") (Target :type "Actor Object Reference"))
  (bind _returnvalue (`|SpawnActorFromClass` "/Game/TestFolder/SimpleProjectile/BP_Tier1_Projectile.BP_Tier1_Projectile_C" SpawnTransform "Undefined" "MultiplyWithRoot" (`self.GetOwner`) Target 2000.0 0.0 null))
  (add `/Game/TestFolder/SimpleProjectile/BP_ProjectileBase.OnProjectileImpact` _returnvalue (delegate `OnImpact`)))

(event `OnImpact`
  (params (OtherActor :type "Actor Object Reference") (`Hit Result` :type "HitResult Structure"))
  (bind _returnvalue (`GameplayStatics.ApplyDamage` OtherActor 50.0))
  (`self.OnAttackEnded`)
  (`KismetSystemLibrary.PrintString` (`KismetStringLibrary.Conv_DoubleToString` _returnvalue)))

(event `LaunchFist`
  (params (Target :type "Actor Object Reference") (SpawnTransform :type "Transform Structure"))
  (bind _returnvalue (`|SpawnActorFromClass` "/Game/TestFolder/SimpleProjectile/BP_Fist.BP_Fist_C" SpawnTransform "Undefined" "MultiplyWithRoot" (`self.GetOwner`) Target 1500.0 0.0 null))
  (add `/Game/TestFolder/SimpleProjectile/BP_ProjectileBase.OnProjectileImpact` _returnvalue (delegate `FistImpact`)))

(event `FistImpact`
  (params (OtherActor :type "Actor Object Reference") (`Hit Result` :type "HitResult Structure"))
  (bind _returnvalue (`GameplayStatics.ApplyDamage` OtherActor 50.0))
  (`self.OnAttackEnded`)
  (`KismetSystemLibrary.PrintString` (`KismetStringLibrary.Conv_DoubleToString` _returnvalue)))