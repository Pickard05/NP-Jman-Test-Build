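; BP_Table is a table that tips over when the player kicks it from either side.
; Overlapping Box1 or Box2 binds the player's kick event to a right or left tip, sets IsPushed and disables physics on Top.
; Each tip applies an upward impulse to Top and lerps its rotation through a timeline in opposite directions.
; Box1 only responds once IsPushed is true, while Box2 requires it false.
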(event `self.ReceiveBeginPlay`
  (bind _asplayer (cast `/Game/TestFolder/Player/Player` (`GameplayStatics.GetPlayerCharacter` 0)))
  (set `self.As Player` _asplayer))

(event `self.Box1.OnComponentBeginOverlap`
  (params (OverlappedComponent :type "PrimitiveComponent Object Reference") (OtherActor :type "Actor Object Reference") (OtherComp :type "PrimitiveComponent Object Reference") (OtherBodyIndex :type Integer) (bFromSweep :type Boolean) (SweepResult :type "HitResult Structure (by ref)"))
  (bind _as_player (`self.As Player`))
  (if (== OtherActor _as_player)
    (if (`self.Is Pushed`)
      (add `/Game/TestFolder/Player/Player.OnKickTable` _as_player (delegate `TipTableRight`))
      (set `self.Is Pushed` true)
      (`PrimitiveComponent.SetSimulatePhysics` (`self.Top`) false))))

(event `TipTableRight`
  (`KismetSystemLibrary.PrintString` "Hello")
  (`PrimitiveComponent.AddImpulse` (`self.Top`) (0.0 0.0 100.0) "None" true)
  (bind (_direction _rotatetop) (`Timeline|Box1Hit`)
    (:`Update`
      (`SceneComponent.K2_SetRelativeRotation` (`self.Top`) (`KismetMathLibrary.RLerp` (struct) (struct :`Roll` -60.0) _rotatetop) false false))))

(event `self.Box2.OnComponentBeginOverlap`
  (params (OverlappedComponent :type "PrimitiveComponent Object Reference") (OtherActor :type "Actor Object Reference") (OtherComp :type "PrimitiveComponent Object Reference") (OtherBodyIndex :type Integer) (bFromSweep :type Boolean) (SweepResult :type "HitResult Structure (by ref)"))
  (bind _as_player (`self.As Player`))
  (if (== OtherActor _as_player)
    (if (not (`self.Is Pushed`))
      (add `/Game/TestFolder/Player/Player.OnKickTable` _as_player (delegate `TipTableLeft`))
      (set `self.Is Pushed` true)
      (`PrimitiveComponent.SetSimulatePhysics` (`self.Top`) false))))

(event `TipTableLeft`
  (`KismetSystemLibrary.PrintString` "Hello")
  (`PrimitiveComponent.AddImpulse` (`self.Top`) (0.0 0.0 100.0) "None" true)
  (bind (_direction _rotatetop) (`Timeline|Box2Hit`)
    (:`Update`
      (`SceneComponent.K2_SetRelativeRotation` (`self.Top`) (`KismetMathLibrary.RLerp` (struct) (struct :`Roll` 60.0) _rotatetop) false false))))

(fn `UserConstructionScript`)